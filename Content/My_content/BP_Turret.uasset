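; BP_Turret is a turret actor that fires repeatedly from its Sphere component's transform and can track the player.
; BeginPlay picks single Bullet shots or a scatter burst with random yaw spread, each repeating itself after a FireRate delay.
; When LookAT is set, Tick turns the whole actor toward the player pawn, with FireUpward scaling both heights to control vertical aim.
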(event Custom|Following
  (bind _returnvalue (Game|Player|GetPlayerPawn 0))
  (bind _returnvalue_2 (Transformation|GetActorLocation))
  (bind _returnvalue_3 (Transformation|GetActorLocation _returnvalue))
  (if (Variables|Default|GetLookAT)
    (Transformation|SetActorRotation (Math|Rotator|FindLookatRotation (Math|Vector|MakeVector (.x _returnvalue_2) (.y _returnvalue_2) (* (.z _returnvalue_2) (Variables|Default|GetFireUpward))) (Math|Vector|MakeVector (.x _returnvalue_3) (.y _returnvalue_3) (* (.z _returnvalue_3) (Variables|Default|GetFireUpward)))))))

(event Custom|Shoot
  (Game|SpawnActorfromClass "/Game/My_content/Bullet.Bullet_C" (Transformation|GetSocketTransform (Variables|Default|GetSphere) "None" "RTS_World") "Undefined" "MultiplyWithRoot" 0 0)
  (Utilities|FlowControl|Delay (Variables|Default|GetFireRate))
  (CallFunction|Shoot))

(event Custom|ScatterShot
  (bind _sphere (Variables|Default|GetSphere))
  (bind _returnvalue (Transformation|GetSocketTransform _sphere "None" "RTS_World"))
  (for _index (range 0 3)
    (Game|SpawnActorfromClass "/Game/My_content/Bullet.Bullet_C" (Math|Transform|MakeTransform (.location _returnvalue) (Math|Rotator|MakeRotator (.roll (.rotation _returnvalue)) (.pitch (.rotation _returnvalue)) (+ (.yaw (.rotation _returnvalue)) (Math|Random|RandomFloatinRange -3e+01 3e+01)))) "Undefined" "MultiplyWithRoot" 0 0))
  (Utilities|FlowControl|Delay (Variables|Default|GetFireRate))
  (CallFunction|ScatterShot))

(event EventBeginPlay
  (if (Variables|Default|GetScatter)
    (CallFunction|ScatterShot)
    (else
      (CallFunction|Shoot))))

(event Collision|EventActorBeginOverlap
  (params (OtherActor :type Actor%20Object%20Reference)))

(event EventTick
  (params (DeltaSeconds :type Float%20%28single-precision%29))
  (CallFunction|Following))

(fn ConstructionScript)