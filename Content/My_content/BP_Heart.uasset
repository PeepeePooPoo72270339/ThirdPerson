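; BP_Heart is a falling heart actor that disappears when the player touches it.
; While CanFall is true, Tick lowers it by a fixed step each frame without sweeping or scaling by delta time, so fall speed depends on frame rate.
; Overlapping an actor tagged Platform clears CanFall to stop the fall.
; Overlapping a Player-tagged actor destroys the heart, with no health or score change in this Blueprint.
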(event Collision|EventActorBeginOverlap
  (params (OtherActor :type Actor%20Object%20Reference))
  (if (Actor|ActorHasTag OtherActor "Player")
    (Actor|DestroyActor)
    (elif (Actor|ActorHasTag OtherActor "Platform")
      (Variables|Default|SetCan%20fall? false))))

(event EventTick
  (params (DeltaSeconds :type Float%20%28single-precision%29))
  (if (Variables|Default|GetCan%20fall?)
    (Transformation|SetActorLocation (- (Transformation|GetActorLocation) "0.000000,0.000000,2.000000") false false)))

(fn ConstructionScript)