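; BP_NPC is an NPC actor that plays a sequence of dialogue lines through the player character when overlapped.
; Any overlapping actor triggers DialogReset, as the Player tag check is unconnected, restarting the Dialogue array from its first entry.
; DialogUpdate writes the current line to BP_ThirdPersonCharacter's Text, then calls itself after a fixed Delay until the array ends, ignoring its NextText input.
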(event Custom|DialogUpdate
  (params (NextText :type String))
  (bind _output_get (Variables|Default|SetCurrent_DialogueText (Utilities|Array|Get(acopy) (Variables|Default|GetDialogue) (Variables|Default|GetCurrent))))
  (bind _asbp_third_person_character (Utilities|Casting|CastToBP_ThirdPersonCharacter (Game|GetPlayerCharacter 0)))
  (Variables|/Game/ThirdPerson/Blueprints/BP_ThirdPersonCharacter.BP_ThirdPersonCharacter_C|SetText _asbp_third_person_character _output_get)
  (Variables|Default|SetCurrent (+ (Variables|Default|GetCurrent) 1))
  (Utilities|FlowControl|Delay 3.0)
  (if (!= (Variables|Default|GetCurrent) (Utilities|Array|Length (Variables|Default|GetDialogue)))
    (CallFunction|DialogUpdate)))

(event Custom|DialogReset
  (Variables|Default|SetCurrent 0)
  (CallFunction|DialogUpdate))

(event EventBeginPlay)

(event Collision|EventActorBeginOverlap
  (params (OtherActor :type Actor%20Object%20Reference))
  (if true
    (CallFunction|DialogReset)))

(event EventTick
  (params (DeltaSeconds :type Float%20%28single-precision%29)))

(fn ConstructionScript)