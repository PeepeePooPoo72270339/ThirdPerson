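; BP_FallingPlatform is a platform that vanishes when stepped on and reappears after a short delay, with no falling motion.
; The Collision component's overlap events set PlayerOnTop without checking which actor overlapped.
; While the flag is true, Tick hides SMPlatform and disables its collision, then a Delay restores both.
; Timer resets on both overlap events, but its increment is disconnected, so it has no effect.
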(event OnComponentEndOverlap(Collision)
  (params (OverlappedComponent :type Primitive%20Component%20Object%20Reference) (OtherActor :type Actor%20Object%20Reference) (OtherComp :type Primitive%20Component%20Object%20Reference) (OtherBodyIndex :type Integer))
  (Variables|Default|SetPlayerOnTop false)
  (Variables|Default|SetTimer 0.0))

(event OnComponentBeginOverlap(Collision)
  (params (OverlappedComponent :type Primitive%20Component%20Object%20Reference) (OtherActor :type Actor%20Object%20Reference) (OtherComp :type Primitive%20Component%20Object%20Reference) (OtherBodyIndex :type Integer) (bFromSweep :type Boolean) (SweepResult :type Hit%20Result%20Structure%20%28by%20ref%29))
  (Variables|Default|SetPlayerOnTop true)
  (Variables|Default|SetTimer 0.0))

(event Collision|EventActorBeginOverlap
  (params (OtherActor :type Actor%20Object%20Reference)))

(event EventTick
  (params (DeltaSeconds :type Float%20%28single-precision%29))
  (if (Variables|Default|GetPlayerOnTop)
    (Rendering|SetVisibility (Variables|Default|GetSM_Platform) false false)
    (Collision|SetCollisionEnabled (Variables|Default|GetSM_Platform) "NoCollision")
    (Utilities|FlowControl|Delay 2.0)
    (Rendering|SetVisibility (Variables|Default|GetSM_Platform) true false)
    (Collision|SetCollisionEnabled (Variables|Default|GetSM_Platform) "QueryAndPhysics")))

(fn ConstructionScript)